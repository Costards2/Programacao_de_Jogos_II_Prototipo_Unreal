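; Coin pickup actor that adds to the player's gem count and score, then removes itself.
; On any actor overlap it casts player pawn 0 to Player, without checking which actor overlapped, and increments Gemas and Score directly.
; It then destroys its Spite component and the actor; if the cast fails, nothing happens.
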(event Collision|EventActorBeginOverlap
  (params (OtherActor :type Actor%20Object%20Reference))
  (bind _asplayer (Utilities|Casting|CastToPlayer (Game|Player|GetPlayerPawn 0)))
  (Variables|/Game/BluePrints/Player.Player_C|SetGemas _asplayer (+ (Variables|/Game/BluePrints/Player.Player_C|GetGemas _asplayer) 1))
  (Variables|/Game/BluePrints/Player.Player_C|SetScore _asplayer (+ (Variables|/Game/BluePrints/Player.Player_C|GetScore _asplayer) 100))
  (Components|DestroyComponent (Variables|Default|Getspite))
  (Actor|DestroyActor))

(fn ConstructionScript)