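; Frog enemy Blueprint that can be squashed and removed from the game.
; A capsule hit near the SquashPoint component disables collision, flattens and lowers the sprite, then a short timer destroys the actor.
; The hit check compares only impact location, without filtering which actor hit it.
; Logic to destroy a colliding Player exists but is disconnected, so it never runs.
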(event OnComponentHit(CapsuleComponent)
  (params (HitComponent :type Primitive%20Component%20Object%20Reference) (OtherActor :type Actor%20Object%20Reference) (OtherComp :type Primitive%20Component%20Object%20Reference) (NormalImpulse :type Vector :default "0, 0, 0") (Hit :type Hit%20Result%20Structure%20%28by%20ref%29))
  (bind _sprite (Variables|Default|GetSprite))
  (bind _relativescale3d (Variables|/Script/Engine.SceneComponent|GetRelativeScale3D _sprite))
  (if (Utilities|Operators|EqualEqual (.ImpactPoint (Collision|BreakHitResult Hit)) (Transformation|GetWorldLocation (Variables|Default|GetSquashPoint)) 5e+01)
    (Collision|SetCollisionEnabled (Variables|Collision|GetCapsuleComponent) "NoCollision")
    (Transformation|SetRelativeScale3D _sprite (Math|Vector|MakeVector (.x _relativescale3d) (.y _relativescale3d) (/ (.z _relativescale3d) 2.0)))
    (Transformation|AddLocalOffset _sprite "0.000000,0.000000,-5.000000" false true)
    (Utilities|Time|SetTimerbyEvent (delegate Custom|Squished) 1.0)))

(event Custom|Squished
  (Actor|DestroyActor))

(event EventBeginPlay)

(event Collision|EventActorBeginOverlap
  (params (OtherActor :type Actor%20Object%20Reference)))

(event EventTick
  (params (DeltaSeconds :type Float%20%28single-precision%29)))

(fn ConstructionScript)