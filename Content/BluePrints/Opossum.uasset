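; Opossum is a patrolling 2D enemy character that can be squashed.
; It moves along its negated forward vector every tick and flips around when its LedgeDetector ends an overlap.
; A capsule hit near SquashPoint, from any actor, disables collision, flattens and lowers the sprite, then destroys it after one second.
; The Player cast and Hit call are unconnected, so it never damages the player.
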(event OnComponentHit(CapsuleComponent)
  (params (HitComponent :type Primitive%20Component%20Object%20Reference) (OtherActor :type Actor%20Object%20Reference) (OtherComp :type Primitive%20Component%20Object%20Reference) (NormalImpulse :type Vector :default "0, 0, 0") (Hit :type Hit%20Result%20Structure%20%28by%20ref%29))
  (bind _sprite (Variables|Default|GetSprite))
  (bind _relativescale3d (Variables|/Script/Engine.SceneComponent|GetRelativeScale3D _sprite))
  (if (Utilities|Operators|EqualEqual (.ImpactPoint (Collision|BreakHitResult Hit)) (Transformation|GetWorldLocation (Variables|Default|GetSquash%20Point%20)) 5e+01)
    (Collision|SetCollisionEnabled (Variables|Collision|GetCapsuleComponent) "NoCollision")
    (Pawn|Input|AddMovementInput "0, 0, 0" 0.0 false)
    (Transformation|SetRelativeScale3D _sprite (Math|Vector|MakeVector (.x _relativescale3d) (.y _relativescale3d) (/ (.z _relativescale3d) 2.0)))
    (Transformation|AddLocalOffset _sprite "0.000000,0.000000,-9.000000" false true)
    (Utilities|Time|SetTimerbyEvent (delegate Custom|Squished) 1.0)))

(event OnComponentEndOverlap(LedgeDetector)
  (params (OverlappedComponent :type Primitive%20Component%20Object%20Reference) (OtherActor :type Actor%20Object%20Reference) (OtherComp :type Primitive%20Component%20Object%20Reference) (OtherBodyIndex :type Integer))
  (CallFunction|TurnChar))

(event Custom|Squished
  (Actor|DestroyActor))

(event EventBeginPlay)

(event Collision|EventActorBeginOverlap
  (params (OtherActor :type Actor%20Object%20Reference)))

(event EventTick
  (params (DeltaSeconds :type Float%20%28single-precision%29))
  (Pawn|Input|AddMovementInput (Transformation|GetActorForwardVector) -1.0 false))

(fn ConstructionScript)

(fn TurnChar
  (Transformation|SetActorRotation (Math|Rotator|CombineRotators (Transformation|GetActorRotation) "0.000000,180.000000,0.000000")))